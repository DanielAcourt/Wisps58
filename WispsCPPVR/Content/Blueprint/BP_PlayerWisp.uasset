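; BP_PlayerWisp is the player's wisp, owning the main UI and tracking sensed and interacting actors.
; BeginPlay binds sense and interact events, then creates UI_Parent with a reference to the wisp.
; Tab toggles the mouse cursor, look input and gameplay or menu Enhanced Input mapping context.
; Interaction queries return empty defaults, hover and AI chat events only print, and the SovereignBridgeSubsystem chat setup is disconnected.
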(event Custom|OnActorSensed_Event
  (params (SensedActor :type Actor%20Object%20Reference))
  ;[0.02861 0.15 0.01604 0.5] Imporant ON Start for the Wisp
  (Variables|Default|SetSensedActor SensedActor))

(event Custom|AiChatPush
  (params (Message :type String))
  ;[0.15 0.001563 0.001563 0.5] xAi Chat System from wisps perspective
  ;;[0.15 0.15 0.15 0.5] Comment
  (Development|PrintString Message))

(event Custom|ListenForNetworkMessages
  ;[0.15 0.1078 0.002673 0.5] Network Messaging
)

(event Custom|MultcastEventMessages
  ;[0.15 0.1078 0.002673 0.5] Network Messaging
  (Default|AddChatMessage (Variables|Default|GetChatWidgetREf) (Utilities|GetDisplayName self)))

(event EventBeginPlay
  ;[0.02861 0.15 0.01604 0.5] Imporant ON Start for the Wisp
  (EventDispatchers|BindEventtoOnActorSensed (delegate Custom|OnActorSensed_Event))
  (CallFunction|SetUi 0 self)
  (EventDispatchers|BindEventtoOnActorInteracted (delegate EventOnInteract)))

(event Collision|EventActorBeginOverlap
  (params (OtherActor :type Actor%20Object%20Reference))
  ;[0.15 0.15 0.15 0.5] Interaction Triggers
)

(event EventTick
  (params (DeltaSeconds :type Float%20%28single-precision%29)))

(event EventOnBeginHover
  ;[0.15 0.15 0.15 0.5] On Hover
  (Development|PrintString "On hover Detected"))

(event EventOnEndHover
  ;[0.15 0.15 0.15 0.5] On Hover
  (Development|PrintString "End Hover Detected"))

(event EventOnInteract
  (params (Interactor :type Actor%20Object%20Reference))
  ;[0.02861 0.15 0.01604 0.5] Imporant ON Start for the Wisp
  (Variables|Default|SetInteractor Interactor))

(event EventOnSecondaryInteract
  (params (Interactor :type Actor%20Object%20Reference))
  ;[0.15 0.15 0.15 0.5] Interaction Triggers
)

(event Input|KeyboardEvents|Tab
  (params (Key :type Key%20Structure :default "None"))
  (:Pressed
    (CallFunction|ShowHideCursor)))

(fn ConstructionScript)

(fn CanInteract
  (params (Interactor :type Actor%20Object%20Reference))
  (return false))

(fn GetInteractionHint
  (return ""))

(fn GetInteractableName
  (return ""))

(fn GetInhabitingSpirit
  (return 0))

(fn SetUi
  (params (InteractedActor :type Actor%20Object%20Reference) (Wisp :type BP%20Player%20Wisp%20Object%20Reference))
  ;[0.15 0.15 0.15 0.5] Comment
  (bind _returnvalue (UserInterface|CreateWidget "/Game/Assets/UI/UI_Parent.UI_Parent_C" 0 0 InteractedActor "/Game/Assets/UI/UI_Parent.Default__UI_Parent_C.WBP_BIO_C_0" 0 0 Wisp 0 0))
  (bind _output_get (Variables|Default|SetMainUiParent _returnvalue))
  (UserInterface|Viewport|AddtoPlayerScreen _output_get)
  (Widget|SetVisibility _output_get "Visible"))

(fn ShowHideCursor
  (bind _returnvalue (Game|GetPlayerController 0))
  (bind _returnvalue_2 (PlayerController|LocalPlayerSubsystems|GetEnhancedInputLocalPlayerSubsystem _returnvalue))
  (if (Variables|Default|GetActiveCursor)
    (Variables|/Script/Engine.PlayerController|SetbShowMouseCursor _returnvalue false)
    (Variables|Default|SetActiveCursor false)
    (Input|SetIgnoreLookInput _returnvalue false)
    (Input|RemoveMappingContext _returnvalue_2 "/Game/Input/IMC_WispsMenu.IMC_WispsMenu" (Utilities|Struct|MakeModifyContextOptions true false false))
    (Input|AddMappingContext _returnvalue_2 "/Game/Input/IMC_Wisp.IMC_Wisp" 0 "(bIgnoreAllPressedKeysUntilRelease=True,bForceImmediately=False,bNotifyUserSettings=False)")
    (else
      (Variables|/Script/Engine.PlayerController|SetbShowMouseCursor _returnvalue true)
      (Variables|Default|SetActiveCursor true)
      (Input|SetIgnoreLookInput _returnvalue true)
      (Input|RemoveMappingContext _returnvalue_2 "/Game/Input/IMC_Wisp.IMC_Wisp" (Utilities|Struct|MakeModifyContextOptions true false false))
      (Input|AddMappingContext _returnvalue_2 "/Game/Input/IMC_WispsMenu.IMC_WispsMenu" 0 "(bIgnoreAllPressedKeysUntilRelease=True,bForceImmediately=False,bNotifyUserSettings=False)"))))