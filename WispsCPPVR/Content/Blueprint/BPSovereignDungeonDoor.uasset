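; Interactable Sovereign dungeon door that swings open and starts a random enemy encounter.
; BeginPlay caches the battle manager from the dungeon game mode.
; On interact, it calls OpenDoor and runs a timeline that rotates the door leaf's yaw.
; The first timeline update with a valid character interactor triggers the encounter subsystem once through a DoOnce, passing the candidate pool, battle manager, random seed and a hardcoded spawn location.
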(event EventBeginPlay
  (bind _assovereign_dungeon_game_mode (Utilities|Casting|CastToSovereignDungeonGameMode (Game|GetGameMode)))
  (Variables|Default|SetBattleManager (Class|SovereignDungeonGameMode|GetBattleManager _assovereign_dungeon_game_mode)))

(event Collision|EventActorBeginOverlap
  (params (OtherActor :type Actor%20Object%20Reference)))

(event EventTick
  (params (DeltaSeconds :type Float%20%28single-precision%29)))

(event EventOnInteract
  (params (Interactor :type Actor%20Object%20Reference))
  (Class|SovereignDungeonDoor|OpenDoor self)
  (bind _rotationrate (Timeline|Timeline PlayFromStart)
    (:Update
      (Transformation|SetRelativeRotation (Variables|Default|GetDoorLeafMeshComponent) (Math|Rotator|MakeRotator 0.0 0.0 _rotationrate) false false)
      (bind _assovereign_base_character (Utilities|Casting|CastToSovereignBaseCharacter Interactor))
      (Utilities|FlowControl|DoOnce false
        (:Completed
          (Class|SovereignEncounterSubsystem|TriggerRandomEncounter (Subsystems|GetSovereignEncounterSubsystem) _assovereign_base_character 0 (Variables|Default|GetCandidate%20Pool) (Utilities|Array|MakeArray (Class|GeometryScriptLibraryTransformFunctions|MakeTransformfromAxes "50100.000000,50100.000000,50100.000000" "0, 0, 0" "0, 0, 0" true)) 20 (Math|Random|RandomInteger 9999) true (Variables|Default|GetBattleManager)))))
    (:Finished
      (Development|PrintString "Finshed opening door"))))

(fn ConstructionScript)