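; Battle manager Blueprint that ties the Sovereign encounter flow to the battle HUD.
; On BeginPlay it binds to its combatant turn-ready event and to the encounter subsystem's transition start and end events.
; Transition start creates and shows a new battle HUD widget with the mouse cursor, and transition end only hides the widget.
; Turn changes only print the combatant's name, and the battle input mapping context is left unconnected.
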(event Custom|OnCombatantTurnReady_Event
  (params (Combatant :type Sovereign%20Base%20Character%20Object%20Reference))
  ;[0.15 0.15 0.15 0.5] Comment
  (Development|PrintString (Utilities|String|Append "whos turn it is in combat" (Utilities|GetDisplayName Combatant))))

(event Custom|OnEncounterTransitionStarted_Event
  (params (BattleManager :type Sovereign%20Battle%20Manager%20Object%20Reference))
  ;[0.15 0.15 0.15 0.5] Comment
  (Development|PrintString (Utilities|String|Append "Battle manager has triggered Start of Encounter" "Might be smarter to render Ui her"))
  (CallFunction|BattleHUDShow))

(event Custom|OnEncounterTransitionEnded_Event
  (params (Outcome :type EBattleState%20Enum :default "EncounterStarting"))
  ;[0.15 0.15 0.15 0.5] Comment
  (Development|PrintString "Battle Manager has detected end of combat")
  (CallFunction|BattleHUDHide))

(event EventBeginPlay
  (bind _returnvalue (Subsystems|GetSovereignEncounterSubsystem))
  (EventDispatchers|AssignOnCombatantTurnReady (delegate Custom|OnCombatantTurnReady_Event))
  (EventDispatchers|AssignOnEncounterTransitionStarted _returnvalue (delegate Custom|OnEncounterTransitionStarted_Event))
  (EventDispatchers|AssignOnEncounterTransitionEnded _returnvalue (delegate Custom|OnEncounterTransitionEnded_Event)))

(event Collision|EventActorBeginOverlap
  (params (OtherActor :type Actor%20Object%20Reference)))

(event EventTick
  (params (DeltaSeconds :type Float%20%28single-precision%29)))

(fn ConstructionScript)

(fn BattleHUDShow
  (bind _returnvalue (UserInterface|CreateWidget "/Game/Assets/UI/BattleUI/WBP_SovereignBattleHUD.WBP_SovereignBattleHUD_C"))
  (bind _output_get (Variables|Default|SetUIMainBattleHUD _returnvalue))
  (UserInterface|Viewport|AddtoPlayerScreen _output_get)
  (Widget|SetVisibility _output_get "Visible")
  (Variables|/Script/Engine.PlayerController|SetbShowMouseCursor (Game|GetPlayerController 0) true))

(fn BattleHUDHide
  (Widget|SetVisibility (Variables|Default|GetUIMainBattleHUD) "Hidden"))