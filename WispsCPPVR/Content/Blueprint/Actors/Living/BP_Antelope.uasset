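; BP_Antelope is a possessable antelope creature that receives Qi from the spirit inhabiting it.
; On possession it finds the inhabiting spirit and tries to spend a fixed amount from that spirit's SovereignQiComponent.
; If the spend succeeds, the antelope's QiComponent absorbs the same amount at full purity.
; Debug prints report the controller and transfer result, unpossession only prints, and BeginPlay, overlap and Tick are unused.
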(event EventBeginPlay
  (|CallParentFunction) ; This node is disabled and will not be called.\nDrag off pins to build functionality.
)

(event Collision|EventActorBeginOverlap
  (params (OtherActor :type Actor%20Object%20Reference))
  (|CallParentFunction OtherActor) ; This node is disabled and will not be called.\nDrag off pins to build functionality.
)

(event EventTick
  (params (DeltaSeconds :type Float%20%28single-precision%29))
  (|CallParentFunction DeltaSeconds) ; This node is disabled and will not be called.\nDrag off pins to build functionality.
)

(event EventPossessed
  (params (NewController :type Controller%20Object%20Reference))
  (Development|PrintString (Utilities|GetDisplayName NewController))
  (bind _returnvalue (Class|InteractionInterface|GetInhabitingSpirit))
  (Utilities|IsValid _returnvalue
    (:Is%20Valid
      (bind _returnvalue_2 (Class|SovereignQiComponent|SpendQi (Actor|GetComponentbyClass _returnvalue "/Script/WispCPP7VR.SovereignQiComponent") 2e+01))
      (if _returnvalue_2
        (Class|SovereignQiComponent|AbsorbQi (Variables|Default|GetQiComponent) 2e+01 1.0)
        (Development|PrintString "able to spend qi")
        (else
          (Development|PrintString "Unable to spend qi"))))
    (:Is%20Not%20Valid
      (Development|PrintString "UNablke to find the correct interface"))))

(event EventUnpossessed
  (params (OldController :type Controller%20Object%20Reference))
  (Development|PrintString (Utilities|GetDisplayName OldController)))

(fn ConstructionScript
  (|CallParentFunction))