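; BP_Dragon is a dragon actor Blueprint whose only active logic is a game mode debug check.
; On BeginPlay it calls the parent, then casts the game mode to SovereignDungeonGameMode and prints its name.
; If that cast fails, it prints a failure and tries SovWispsGameModeBase, printing either that name or an incorrect-after-level-load warning.
; Tick and overlap events are disabled, and the construction script only calls its parent.
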(event EventBeginPlay
  (bind _returnvalue (Game|GetGameMode))
  (|CallParentFunction)
  (bind _assovereign_dungeon_game_mode (Utilities|Casting|CastToSovereignDungeonGameMode _returnvalue)
    (:then
      (Development|PrintString (Utilities|String|Append "My game mode is" (Utilities|GetDisplayName _assovereign_dungeon_game_mode)) true true "(R=0.000000,G=0.000000,B=0.000000,A=1.000000)" 22.0))
    (:CastFailed
      (Development|PrintString (Utilities|String|Append "Game mode failed" "") true true "(R=0.000000,G=0.000128,B=0.033365,A=1.000000)" 22.0)
      (bind _assov_wisps_game_mode_base (Utilities|Casting|CastToSovWispsGameModeBase _returnvalue)
        (:then
          (Development|PrintString (Utilities|String|Append "My game mode is" (Utilities|GetDisplayName _assov_wisps_game_mode_base)) true true "(R=0.000000,G=0.000000,B=0.000000,A=1.000000)" 22.0))
        (:CastFailed
          (Development|PrintString "Game mode is incorrect after level load"))))))

(event Collision|EventActorBeginOverlap
  (params (OtherActor :type Actor%20Object%20Reference))
  (|CallParentFunction OtherActor) ; This node is disabled and will not be called.\nDrag off pins to build functionality.
)

(event EventTick
  (params (DeltaSeconds :type Float%20%28single-precision%29))
  (|CallParentFunction DeltaSeconds) ; This node is disabled and will not be called.\nDrag off pins to build functionality.
)

(fn ConstructionScript
  (|CallParentFunction))