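; An Iron Knight agent actor that voices chat responses through text-to-speech.
; On BeginPlay it subscribes to the Sovereign Bridge subsystem's chat response event, then adds and activates its own channel in the TextToSpeech engine subsystem.
; Each response's content is spoken on that channel.
; A runtime directive call to the bridge and a debug print are left unconnected and never run.
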(event Custom|OnChatResponseReceived_Event
  (params (Response :type Sovereign%20Chat%20Response%20Structure%20%28by%20ref%29))
  (Class|TexttoSpeechEngineSubsystem|SpeakonChannel (|TexttoSpeechEngineSubsystem) (Variables|Default|GetIronKnightChannel) (Utilities|String|ToString(Text) (Utilities|Text|ToText(String) (.Content (Utilities|Struct|BreakSovereignChatResponse Response))))))

(event EventBeginPlay
  (bind _returnvalue (|TexttoSpeechEngineSubsystem))
  (bind _ironknightchannel (Variables|Default|GetIronKnightChannel))
  (EventDispatchers|AssignOnChatResponseReceived (Subsystems|GetSovereignBridgeSubsystem) (delegate Custom|OnChatResponseReceived_Event))
  (Class|TexttoSpeechEngineSubsystem|AddDefaultChannel _returnvalue _ironknightchannel)
  (Class|TexttoSpeechEngineSubsystem|ActivateChannel _returnvalue _ironknightchannel))

(event Collision|EventActorBeginOverlap
  (params (OtherActor :type Actor%20Object%20Reference)))

(event EventTick
  (params (DeltaSeconds :type Float%20%28single-precision%29)))

(fn ConstructionScript)